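; BP_Platform is a lockable moving platform that carries a Cube along a spline path.
; The Move timeline's Duration track scales the spline length into a distance, and each update places the Cube at that world location without sweeping.
; Unlock plays the timeline, while LockIt stops it, as does BeginPlay when the Lock flag is set.
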(event Custom|Unlock
  (bind _spline (Variables|Default|GetSpline))
  (bind _duration (Timeline|Move Play)
    (:Update
      (Transformation|SetWorldLocation (Variables|Default|GetCube) (Spline|GetLocationatDistanceAlongSpline _spline (* _duration (Spline|GetSplineLength _spline)) "World") false false))))

(event Custom|LockIt
  (bind _spline (Variables|Default|GetSpline))
  (bind _duration (Timeline|Move Stop)
    (:Update
      (Transformation|SetWorldLocation (Variables|Default|GetCube) (Spline|GetLocationatDistanceAlongSpline _spline (* _duration (Spline|GetSplineLength _spline)) "World") false false))))

(event EventBeginPlay
  (bind _spline (Variables|Default|GetSpline))
  (if (Variables|Default|Getlock)
    (bind _duration (Timeline|Move Stop)
      (:Update
        (Transformation|SetWorldLocation (Variables|Default|GetCube) (Spline|GetLocationatDistanceAlongSpline _spline (* _duration (Spline|GetSplineLength _spline)) "World") false false)))))

(fn ConstructionScript)